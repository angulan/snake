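; Level generator actor that builds a walled square arena with one of several random block layouts.
; GenerateMap destroys previous meshes, adds the borders, then randomly picks big blocks, a cube grid, four rooms or no interior blocks.
; CreateBlock spawns scaled static mesh components and records each covered grid cell, so GenerateMap can return the occupied positions.
; Tick moves the current camera in a small overhead circle using sine and cosine of elapsed time.
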(event EventBeginPlay)

(event Collision|EventActorBeginOverlap
  (params (OtherActor :type Actor%20Object%20Reference)))

(event EventTick
  (params (DeltaSeconds :type Float%20%28single-precision%29))
  (Variables|Default|SetTimePassed (+ DeltaSeconds (Variables|Default|GetTimePassed)))
  (Transformation|SetActorLocation (Variables|Default|GetCurrentCamera) (Math|Vector|MakeVector (* (Math|Trig|Sin(Radians) (Variables|Default|GetTimePassed)) 1e+02) (* (Math|Trig|Cos(Radians) (Variables|Default|GetTimePassed)) 1e+02) 1.7e+03) false false))

(fn ConstructionScript)

(fn CreateBlock
  (params (Position :type Vector :default "0.000000,0.000000,0.000000") (Scale :type Vector :default "1.000000,1.000000,1.000000"))
  (bind _returnvalue (AddComponent|AddStaticMeshComponent false (Math|Transform|MakeTransform (* (Math|Vector|MakeVector (.x Position) (.y Position) (.z Position)) 1e+02) "0, 0, 0" (Math|Vector|MakeVector (.x Scale) (.y Scale) (.z Scale)))))
  (Utilities|Array|Insert (Variables|Default|GetComponents) _returnvalue)
  (for _index (range 1 (Math|Conversions|ToInteger(Byte) (Class|KismetMathLibrary|Round64 (.x Scale))))
    (for _index_2 (range 1 (Math|Conversions|ToInteger(Byte) (Class|KismetMathLibrary|Round64 (.y Scale))))
      (Utilities|Array|Add (Variables|Default|GetOccupiedPositions) (* (+ (Math|Vector|MakeVector (- (.x Position) (/ (- (.x Scale) -1.0) 2.0)) (- (.y Position) (/ (- (.y Scale) -1.0) 2.0)) 0.0) (Math|Vector|MakeVector (Math|Conversions|ToFloat(Integer) _index) (Math|Conversions|ToFloat(Integer) _index_2) 0.0)) 1e+02))))
  (return _returnvalue))

(fn GenerateMap
  (while (> (Utilities|Array|Length (Variables|Default|GetComponents)) 0)
    (Components|DestroyComponent (Utilities|Array|Get(acopy) (Variables|Default|GetComponents)))
    (Utilities|Array|RemoveIndex (Variables|Default|GetComponents)))
  (Utilities|Array|Clear (Variables|Default|GetOccupiedPositions))
  (CallFunction|CreateMapBorders)
  (if (== (Math|Random|RandomInteger 2) 0)
    (if (== (Math|Random|RandomInteger 2) 0)
      ;[0.15 0.15 0.15 0.5] Level 1: Big Blocks
      (CallFunction|CreateBlock "4.500000,4.500000,0.000000" "2.000000,2.000000,1.000000")
      (CallFunction|CreateBlock "4.500000,-4.500000,0.000000" "2.000000,2.000000,1.000000")
      (CallFunction|CreateBlock "-4.500000,-4.500000,0.000000" "2.000000,2.000000,1.000000")
      (CallFunction|CreateBlock "-4.500000,4.500000,0.000000" "2.000000,2.000000,1.000000")
      (else
        ;[0.15 0.15 0.15 0.5] Level 2: Cube Grid
        (for _index (range 0 3)
          (for _index_2 (range 0 3)
            (CallFunction|CreateBlock (Math|Vector|MakeVector (+ (* (Math|Conversions|ToFloat(Integer) _index_2) 4.0) -6.0) (+ (* (Math|Conversions|ToFloat(Integer) _index) 4.0) -6.0) 0.0) "1.000000,1.000000,1.000000")))))
    (elif (== (Math|Random|RandomInteger 2) 0)
      ;[0.15 0.15 0.15 0.5] Level 3: Four Rooms
      (CallFunction|CreateBlock "-6.000000,0.000000,0.000000" "5.000000,1.000000,1.000000")
      (CallFunction|CreateBlock "0.000000,-6.000000,0.000000" "1.000000,5.000000,1.000000")
      (CallFunction|CreateBlock "6.000000,0.000000,0.000000" "5.000000,1.000000,1.000000")
      (CallFunction|CreateBlock "0.000000,6.000000,0.000000" "1.000000,5.000000,1.000000")))
  (return (Variables|Default|GetOccupiedPositions)))

(fn CreateMapBorders
  (CallFunction|CreateBlock "8.000000,0.000000,0.000000" "1.000000,17.000000,1.000000")
  (CallFunction|CreateBlock "0.000000,8.000000,0.000000" "17.000000,1.000000,1.000000")
  (CallFunction|CreateBlock "-8.000000,0.000000,0.000000" "1.000000,17.000000,1.000000")
  (CallFunction|CreateBlock "0.000000,-8.000000,0.000000" "17.000000,1.000000,1.000000"))