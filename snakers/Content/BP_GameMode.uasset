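; Game mode for a Snake game that runs the main menu, mode selection and game-over screens through shared GameData state.
; Start or restart resets GameData and, for mode indices 2 and up, adds a second local player and positions both pawns.
; GenerateMap copies the level generator's occupied tiles into GameData's walls.
; Tick polls IsGameOver to show the restart UI; SetupBehaviorTree is an empty stub with disconnected AI start logic.
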(event Custom|OnGameModeButtonClick
  (bind _returnvalue (UserInterface|CreateWidget "/Game/WBP_GameModes.WBP_GameModes_C"))
  (bind _output_get (Variables|Default|SetGame%20modes%20UI _returnvalue))
  (UserInterface|Viewport|AddtoViewport _output_get 0)
  (CallFunction|ColorButtons (Variables|Default|GetGame%20modes%20UI)))

(event Custom|OnStartButtonClick
  (bind _gamedata (Variables|Default|GetGameData))
  (Widget|RemovefromParent (Variables|Default|GetMenu%20UI))
  (Widget|RemovefromParent (Variables|Default|GetRestart%20UI))
  (Class|GameData|DestroyPlayer2 _gamedata)
  (if (>= (Variables|/Script/snakers.GameData|GetSelectedGameMode _gamedata) 2)
    (CallFunction|AddPlayer))
  (Class|GameData|DataSetup _gamedata)
  (Variables|/Script/snakers.GameData|SetCurrentState _gamedata 1))

(event Custom|Generate%20Map
  (Utilities|Array|Clear (Variables|/Script/snakers.GameData|GetOccupiedWalls (Variables|Default|GetGameData)))
  (CallFunction|SetupBehaviorTree)
  (bind _outactors (Actor|GetAllActorsOfClass "/Game/BP_LevelGenerator.BP_LevelGenerator_C"))
  (bind _occupiedpositions (Default|GenerateMap (Utilities|Array|Get(acopy) _outactors)))
  (bind _output_get (Variables|Default|SetOccupiedMapTiles _occupiedpositions))
  (for _array_element _output_get
    (Utilities|Array|Insert (Variables|/Script/snakers.GameData|GetOccupiedWalls (Variables|Default|GetGameData)) _array_element)))

(event Collision|EventActorBeginOverlap
  (params (OtherActor :type Actor%20Object%20Reference)))

(event EventBeginPlay
  (Variables|/Script/snakers.GameData|SetCurrentState (Variables|Default|GetGameData) 0)
  (bind _returnvalue (UserInterface|CreateWidget "/Game/WBP_GameOver.WBP_GameOver_C"))
  (Variables|Default|SetRestart%20UI _returnvalue)
  (bind _returnvalue_2 (UserInterface|CreateWidget "/Game/WBP_MainMenu.WBP_MainMenu_C"))
  (bind _output_get (Variables|Default|SetMenu%20UI _returnvalue_2))
  (UserInterface|Viewport|AddtoViewport _output_get 0)
  (Variables|/Script/Engine.PlayerController|SetbShowMouseCursor (Game|GetPlayerController 0) true)
  (EventDispatchers|AssignOnClicked (Variables|/Game/WBP_MainMenu.WBP_MainMenu_C|GetGamemodes (Variables|Default|GetMenu%20UI)) (delegate Custom|OnGameModeButtonClick))
  (EventDispatchers|BindEventtoOnClicked (Variables|/Game/WBP_MainMenu.WBP_MainMenu_C|GetStartbutton_1 (Variables|Default|GetMenu%20UI)) (delegate Custom|OnStartButtonClick)))

(event EventTick
  (params (DeltaSeconds :type Float%20%28single-precision%29))
  (bind _gamedata (Variables|Default|GetGameData))
  (if (Variables|/Script/snakers.GameData|GetIsGameOver _gamedata)
    (Variables|/Script/snakers.GameData|SetCurrentState _gamedata 2)
    (UserInterface|Viewport|AddtoViewport (Variables|Default|GetRestart%20UI) 0)
    (Variables|/Script/Engine.PlayerController|SetbShowMouseCursor (Game|GetPlayerController 0) true)
    (EventDispatchers|BindEventtoOnClicked (Variables|/Game/WBP_GameOver.WBP_GameOver_C|GetRestartButton (Variables|Default|GetRestart%20UI)) (delegate Custom|OnStartButtonClick))))

(fn ConstructionScript)

(fn ColorButtons
  (params (UI :type WBP%20Game%20Modes%20Object%20Reference))
  (bind _output_color (CallFunction|GetColor))
  (Class|Button|SetBackgroundColor (Variables|/Game/WBP_GameModes.WBP_GameModes_C|GetSolobutton UI) _output_color)
  (bind _output_color_2 (CallFunction|GetColor 1))
  (Class|Button|SetBackgroundColor (Variables|/Game/WBP_GameModes.WBP_GameModes_C|GetSoloAIbutton UI) _output_color_2)
  (bind _output_color_3 (CallFunction|GetColor 2))
  (Class|Button|SetBackgroundColor (Variables|/Game/WBP_GameModes.WBP_GameModes_C|GetPvPbutton UI) _output_color_3)
  (bind _output_color_4 (CallFunction|GetColor 3))
  (Class|Button|SetBackgroundColor (Variables|/Game/WBP_GameModes.WBP_GameModes_C|GetPvAIbutton UI) _output_color_4)
  (bind _output_color_5 (CallFunction|GetColor 4))
  (Class|Button|SetBackgroundColor (Variables|/Game/WBP_GameModes.WBP_GameModes_C|GetAIvAIbutton UI) _output_color_5))

(fn GetColor
  (params (ButtonIndex :type Integer))
  (if (== ButtonIndex (Variables|/Script/snakers.GameData|GetSelectedGameMode (Variables|Default|GetGameData)))
    (return "(R=0.063832,G=0.135202,B=1.000000,A=1.000000)")
    (else
      (return "(R=1.000000,G=1.000000,B=1.000000,A=1.000000)"))))

(fn SetSelectedButton
  (params (Index :type Integer))
  (Variables|/Script/snakers.GameData|SetSelectedGameMode (Variables|Default|GetGameData) Index)
  (CallFunction|ColorButtons (Variables|Default|GetGame%20modes%20UI)))

(fn SetupBehaviorTree)

(fn AddPlayer
  (if (== (Class|GameplayStatics|GetNumPlayerControllers) 2)
    (Class|GameplayStatics|RemovePlayer (Game|GetPlayerController 1) false))
  (Transformation|SetActorLocation (Game|Player|GetPlayerPawn 0) "-300.000000,300.000000,50.000000" false false)
  (bind _returnvalue (Class|GameplayStatics|CreatePlayer 1))
  (bind _assnake (Utilities|Casting|CastToSnake (Game|Player|GetPlayerPawn 1))
    (:then
      (Utilities|Array|Add (Variables|/Script/snakers.GameData|Getsnakes (Variables|Default|GetGameData)) _assnake)
      (Transformation|SetActorLocation _assnake "300.000000,-300.000000,50.000000" false false))
    (:CastFailed
      (Development|PrintText "aww"))))